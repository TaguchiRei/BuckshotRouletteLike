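; Magazine Blueprint for the gun system that builds a randomly ordered load of live bullets and blanks.
; Reload picks random counts from BulletArray and BlankArray, with both index ranges based on BulletArray's length.
; It appends true for each bullet and false for each blank to the Magazine array without clearing it, then shuffles.
; The first entries, up to the newly added count, are printed for debugging.
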(event `Reload`
  (set `self.Bullet` (`|GetArrayItem` (`self.BulletArray`) (`KismetMathLibrary.RandomIntegerInRange` 0 (- (`KismetArrayLibrary.Array_Length` (`self.BulletArray`)) 1))))
  (set `self.Blank` (`|GetArrayItem` (`self.BlankArray`) (`KismetMathLibrary.RandomIntegerInRange` 0 (- (`KismetArrayLibrary.Array_Length` (`self.BulletArray`)) 1))))
  (for _ (range 1 (+ (`self.Bullet`) 1))
    (`KismetArrayLibrary.Array_Add` (`self.Magazine`) true))
  (for _ (range 1 (+ (`self.Blank`) 1))
    (`KismetArrayLibrary.Array_Add` (`self.Magazine`)))
  (`KismetArrayLibrary.Array_Shuffle` (`self.Magazine`))
  (for _index (range (+ (`self.Bullet`) (`self.Blank`)))
    (if (`|GetArrayItem` (`self.Magazine`) _index)
      (`KismetSystemLibrary.PrintString` "Bullet")
      (else
        (`KismetSystemLibrary.PrintString` "Blank")))))

(fn `UserConstructionScript`)