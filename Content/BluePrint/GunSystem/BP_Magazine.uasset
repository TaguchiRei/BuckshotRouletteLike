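; BP_Magazine is a gun magazine holding a random, shuffled mix of live rounds and blanks as a boolean array.
; Reload plays a sound, picks live and blank counts independently from preset arrays (both indices bounded by BulletArray's length), rebuilds and shuffles the magazine, then prints its order for debugging.
; GetNextBullet removes the first round, returning its type and whether it was last.
; CountBullet tallies remaining live and blank rounds.
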(event `Reload`
  (`GameplayStatics.PlaySound2D` "/Game/Audio/Sound/銃のリロード.銃のリロード" 1.0 1.0 0.0 null null)
  (`KismetArrayLibrary.Array_Clear` (`self.Magazine`))
  (set `self.Bullet` (`|GetArrayItem` (`self.BulletArray`) (`KismetMathLibrary.RandomIntegerInRange` 0 (- (`KismetArrayLibrary.Array_Length` (`self.BulletArray`)) 1))))
  (set `self.Blank` (`|GetArrayItem` (`self.BlankArray`) (`KismetMathLibrary.RandomIntegerInRange` 0 (- (`KismetArrayLibrary.Array_Length` (`self.BulletArray`)) 1))))
  (for _ (range 1 (+ (`self.Bullet`) 1))
    (`KismetArrayLibrary.Array_Add` (`self.Magazine`) true))
  (for _ (range 1 (+ (`self.Blank`) 1))
    (`KismetArrayLibrary.Array_Add` (`self.Magazine`)))
  (`KismetArrayLibrary.Array_Shuffle` (`self.Magazine`))
  (`self.MagazineLog`))

(event `MagazineLog`
  (for _index (range (+ (`self.Bullet`) (`self.Blank`)))
    (if (`|GetArrayItem` (`self.Magazine`) _index)
      (`KismetSystemLibrary.PrintString` "Bullet")
      (else
        (`KismetSystemLibrary.PrintString` "Blank")))))

(fn `CountBullet`
  (returns (BulletCount :type Integer) (BlankCount :type Integer))
  (locals (BulletCounter :type Integer))
  (bind _magazine (`self.Magazine`))
  (bind _bulletcounter (`local.BulletCounter`))
  (for _array_element _magazine
    (if _array_element
      (set `local.BulletCounter` (+ (`local.BulletCounter`) 1))))
  (return _bulletcounter (- (`KismetArrayLibrary.Array_Length` _magazine) _bulletcounter)))

(fn `GetNextBullet`
  (returns (Bullet :type Boolean) (LastBullet :type Boolean))
  (locals (FirstBullet :type Boolean))
  (bind _returnvalue (`KismetArrayLibrary.Array_Length` (`self.Magazine`)))
  (bind _output_get (set `local.FirstBullet` (`|GetArrayItem` (`self.Magazine`))))
  (`KismetArrayLibrary.Array_Remove` (`self.Magazine`))
  (`KismetSystemLibrary.PrintString` (`KismetStringLibrary.Concat_StrStr` (`KismetStringLibrary.Conv_IntToString` _returnvalue) "Remove後の球の数LastBulletの値"))
  (return _output_get (== _returnvalue 0)))

(fn `UserConstructionScript`)