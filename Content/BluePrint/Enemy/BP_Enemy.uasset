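; Enemy Blueprint that plays a procedural knock-down and get-up reaction when DamageReaction is triggered.
; DamageReaction waits through a short Delay, then sets the reaction flags and resets the timer.
; Tick lerps actor pitch to -90 over FallSpeed, then back to upright over ReturnSpeed, both acting as durations in seconds.
; The rotation is set absolutely, so yaw and roll are zeroed during the reaction.
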(event `self.ReceiveBeginPlay`)

(event `self.ReceiveTick`
  (params (DeltaSeconds :type "Float (single-precision)"))
  (bind _returnvalue (/ (`self.CurrentTime`) (`self.ReturnSpeed`)))
  (bind _returnvalue_2 (/ (`self.CurrentTime`) (`self.FallSpeed`)))
  (if (`self.Reaction`)
    (set `self.CurrentTime` (+ (`self.CurrentTime`) DeltaSeconds))
    (if (`self.Downning`)
      (`self.K2_SetActorRotation` (`KismetMathLibrary.MakeRotator` 0.0 (`KismetMathLibrary.Lerp` 0.0 -90.0 _returnvalue_2)))
      (if (> _returnvalue_2 1.0)
        (set `self.CurrentTime` 0.0)
        (set `self.Downning` false))
      (else
        (`self.K2_SetActorRotation` (`KismetMathLibrary.MakeRotator` 0.0 (`KismetMathLibrary.Lerp` -90.0 0.0 _returnvalue)))
        (if (> _returnvalue 1.0)
          (set `self.Reaction` false))))))

(event `DamageReaction`
  (`KismetSystemLibrary.Delay` 0.2)
  (set `self.Downning` true)
  (set `self.Reaction` true)
  (set `self.CurrentTime` 0.0))

(fn `UserConstructionScript`)