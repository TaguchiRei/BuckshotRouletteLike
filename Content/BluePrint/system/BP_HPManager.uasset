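; BP_HPManager is an Actor that holds and adjusts current HP for both the player and an enemy.
; Damage and DamageEnemy subtract from the matching HP and return whether it has reached zero or below.
; HPUP and HPUPEnemy add HP only while it is below the maximum, without clamping, so healing can overshoot.
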(event `HPUPEnemy`
  (params (Amount :type Integer))
  (if (< (`self.EnemyCurrnentHP`) (`self.EnemyHP`))
    (set `self.EnemyCurrnentHP` (+ (`self.EnemyCurrnentHP`) Amount))))

(event `HPUP`
  (params (amount :type Integer))
  (if (< (`self.PlayerCurrnentHPt`) (`self.PlayerHP`))
    (set `self.PlayerCurrnentHPt` (+ (`self.PlayerCurrnentHPt`) amount))))

(fn `Damage`
  (params (DamageNum :type Integer))
  (returns (IsDead :type Boolean))
  (bind _output_get (set `self.PlayerCurrnentHPt` (- (`self.PlayerCurrnentHPt`) DamageNum)))
  (return (<= _output_get 0)))

(fn `DamageEnemy`
  (params (DamageNum :type Integer))
  (returns (IsDead :type Boolean))
  (bind _output_get (set `self.EnemyCurrnentHP` (- (`self.EnemyCurrnentHP`) DamageNum)))
  (return (<= _output_get 0)))

(fn `UserConstructionScript`)