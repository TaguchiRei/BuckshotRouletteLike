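; Player controller for a mouse-driven game in which the player uses items or fires a gun at themselves or the enemy.
; On BeginPlay it switches to the level camera and creates the in-game UI, binding both shot buttons to CallPlayerGunShot.
; Left-click release, gated by InputState.CanInput, traces under the cursor to use an item or, on the magazine, show the shot buttons.
; InvokeDamageEffect relays damage feedback to the UI.
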(event `ShotSelfButton_イベント`
  (`self.PlayerGunShot` true)
  (`Widget.SetVisibility` (`/Game/BluePrint/system/WBP_InGameUI.PlayerButton` (stale `self.ReceiveBeginPlay` _returnvalue_2)) "Hidden" :!label _label)
  (`Widget.SetVisibility` (`/Game/BluePrint/system/WBP_InGameUI.EnemyButton` (stale `self.ReceiveBeginPlay` _returnvalue_2)) "Hidden"))

(event `ShotEnemyButton_イベント`
  (`self.PlayerGunShot` false)
  (goto _label))

(event `self.ReceiveBeginPlay`
  (set `self.bEnableMouseOverEvents` true)
  (set `self.bEnableClickEvents` true)
  (set `self.bShowMouseCursor` true)
  (bind _returnvalue (`GameplayStatics.GetActorOfClass` "/Script/Engine.CameraActor"))
  (`self.SetViewTargetWithBlend` self _returnvalue 0.0 "VTBlend_Linear" 0.0 false)
  (bind _returnvalue_2 (`|CreateWidget` "/Game/BluePrint/system/WBP_InGameUI.WBP_InGameUI_C" (`GameplayStatics.GetPlayerController` 0)))
  (bind _output_get (set `self.InGameUI` _returnvalue_2))
  (`UserWidget.AddToViewport` _output_get 0)
  (`WidgetBlueprintLibrary.SetInputMode_GameOnly` self true)
  (`Widget.SetVisibility` (`/Game/BluePrint/system/WBP_InGameUI.ItemName` _returnvalue_2) "Hidden")
  (`Widget.SetVisibility` (`/Game/BluePrint/system/WBP_InGameUI.ItemInfo` _returnvalue_2) "Hidden")
  (`Widget.SetVisibility` (`/Game/BluePrint/system/WBP_InGameUI.EnemyButton` _returnvalue_2) "Hidden")
  (`Widget.SetVisibility` (`/Game/BluePrint/system/WBP_InGameUI.PlayerButton` _returnvalue_2) "Hidden")
  (`Widget.SetVisibility` (`/Game/BluePrint/system/WBP_InGameUI.DamageEffectImage` _returnvalue_2) "Hidden")
  (add `/Game/BluePrint/system/WBP_InGameUI.ShotSelfButton` _returnvalue_2 (delegate `ShotSelfButton_イベント`))
  (add `/Game/BluePrint/system/WBP_InGameUI.ShotEnemyButton` _returnvalue_2 (delegate `ShotEnemyButton_イベント`))
  (`KismetSystemLibrary.PrintString` "プレイヤーコントローラー初期化完了"))

(event `Key|LeftMouseButton`
  (params (Key :type "Key Structure"))
  (bind _ingameui (`self.InGameUI`))
  (bind (_bblockinghit _binitialoverlap _time _distance _location _impactpoint _normal _impactnormal _physmat _hitactor) (`GameplayStatics.BreakHitResult` (`self.GetHitResultUnderCursorByChannel` "TraceTypeQuery1" false)))
  (:`Pressed`
    (bind _returnvalue (`GameplayStatics.GetActorOfClass` "/Game/BluePrint/system/InputState.InputState_C")))
  (:`Released`
    (if (`/Game/BluePrint/system/InputState.CanInput` _returnvalue)
      (bind _asbp_item_base (cast `/Game/BluePrint/Item/BP_ItemBase` _hitactor)
        (:`then`
          (`KismetSystemLibrary.PrintString` "Get Item")
          (set `/Game/BluePrint/system/InputState.CanInput` false _returnvalue)
          (bind _returnvalue_2 (`GameplayStatics.GetActorOfClass` "/Game/BluePrint/system/InputState.InputState_C"))
          (if (`/Game/BluePrint/system/InputState.UseAdrenaline` _returnvalue_2)
            (set `/Game/BluePrint/system/InputState.UseAdrenaline` false _returnvalue_2))
          (`/Game/BluePrint/Item/BP_ItemBase.UseItem` _asbp_item_base true))
        (:`CastFailed`
          (cast `/Game/BluePrint/GunSystem/BP_Magazine` _hitactor
            (:`then`
              (`KismetSystemLibrary.PrintString` "SelectGun")
              (bind _returnvalue_3 (`GameplayStatics.GetActorOfClass` "/Game/BluePrint/system/InputState.InputState_C"))
              (set `/Game/BluePrint/system/InputState.CanInput` false _returnvalue_3)
              (`Widget.SetVisibility` (`/Game/BluePrint/system/WBP_InGameUI.PlayerButton` _ingameui) "Visible")
              (`Widget.SetVisibility` (`/Game/BluePrint/system/WBP_InGameUI.EnemyButton` _ingameui) "Visible"))
            (:`CastFailed`
              (`KismetSystemLibrary.PrintString` "THIS IS NOT ITEM"))))))))

(event `InvokeDamageEffect`
  (`/Game/BluePrint/system/WBP_InGameUI.DamageEffect` (`self.InGameUI`)))

(fn `UserConstructionScript`)