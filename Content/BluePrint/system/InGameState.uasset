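; In-game state Blueprint running a Buckshot Roulette-style duel: rounds, alternating player and dealer turns, and shot outcomes.
; It coordinates the magazine, item, HP and input actors, resetting them each round.
; Player shots arrive through a controller event; a blank self-shot grants another turn, and handcuffs skip the dealer's turn.
; The dealer uses an item, then ShotEnemy targets the player or itself by comparing live and blank counts.
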(event `self.ReceiveBeginPlay`
  (set `self.State` "NewEnumerator2")
  (set `self.IsMovingGameState` false)
  (set `self.CurrentRound` -1)
  (set `self.MaxRound` 3))

(event `OnInitialized`
  (bind _returnvalue (`GameplayStatics.GetActorOfClass` "/Game/BluePrint/Item/BP_ItemManager.BP_ItemManager_C"))
  (set `self.ItemManager` _returnvalue)
  (bind _returnvalue_2 (`GameplayStatics.GetActorOfClass` "/Game/BluePrint/GunSystem/BP_Magazine.BP_Magazine_C"))
  (set `self.Magazine` _returnvalue_2)
  (bind _returnvalue_3 (`GameplayStatics.GetActorOfClass` "/Game/BluePrint/system/BP_HPManager.BP_HPManager_C"))
  (set `self.HPManager` _returnvalue_3)
  (set `self.State` "NewEnumerator0")
  (bind _returnvalue_4 (`GameplayStatics.GetActorOfClass` "/Game/BluePrint/system/InputState.InputState_C"))
  (set `self.InputState` _returnvalue_4)
  (`self.StartRound`)
  (bind _asbp_uiplayer_controller (cast `/Game/BluePrint/system/BP_UIPlayerController` (`GameplayStatics.GetPlayerController` 0)))
  (add `/Game/BluePrint/system/BP_UIPlayerController.PlayerGunShot` _asbp_uiplayer_controller (delegate `PlayerGunSHot`))
  (`KismetSystemLibrary.PrintString` "GameState初期化完了"))

(event `PlayerGunSHot`
  (params (Target :type Boolean))
  (bind _hpmanager (`self.HPManager`))
  (bind _damagevalue (`/Game/BluePrint/system/InputState.DamageValue` (`self.InputState`)))
  ; プレイヤーが射撃したときに実行するカスタムイベント
  (set `/Game/BluePrint/system/InputState.CanInput` false (`self.InputState`))
  (bind (_bullet _lastbullet) (`/Game/BluePrint/GunSystem/BP_Magazine.GetNextBullet` (`self.Magazine`)))
  (if _bullet
    ;; 実包時の処理
    (`GameplayStatics.PlaySound2D` "/Game/Audio/Sound/拳銃を撃つ.拳銃を撃つ" 1.0 1.0 0.0 null null)
    (if Target
      (bind _asbp_uiplayer_controller (cast `/Game/BluePrint/system/BP_UIPlayerController` (`GameplayStatics.GetPlayerController` 0)))
      (`/Game/BluePrint/system/BP_UIPlayerController.InVokeDamageEffect` _asbp_uiplayer_controller)
      (bind _isdead (`/Game/BluePrint/system/BP_HPManager.Damage` _hpmanager _damagevalue))
      (if _isdead
        (`self.PlayerHPZero` :!label _label)
        (else
          (set `/Game/BluePrint/system/InputState.DamageValue` 1 (`self.InputState`) :!label _label_2)
          (if _lastbullet
            (`self.StartRound`)
            (else
              (`self.StartEnemyTurn`)))))
      (else
        (bind _isdead_2 (`/Game/BluePrint/system/BP_HPManager.DamageEnemy` _hpmanager _damagevalue))
        (if _isdead_2
          (`self.EnemyHPZero` :!label _label_3)
          (else
            (bind _returnvalue (`GameplayStatics.GetActorOfClass` "/Game/BluePrint/Enemy/BP_Enemy.BP_Enemy_C"))
            (`/Game/BluePrint/Enemy/BP_Enemy.DamageReaction` _returnvalue)
            (goto _label_2)))))
    (else
      ;; 空砲時の処理
      (`GameplayStatics.PlaySound2D` "/Game/Audio/Sound/銃火器・空撃ち.銃火器・空撃ち" 1.0 1.0 0.0 null null)
      (if Target
        (`self.StartPlayerTurn`)
        (else
          (goto _label_2))))))

(event `StartRound`
  ; ラウンド開始時のイベント
  (bind _output_get (set `self.CurrentRound` (+ (`self.CurrentRound`) 1)))
  (`/Game/BluePrint/Item/BP_ItemManager.ReplaceAllItem` (`self.ItemManager`) _output_get)
  (`/Game/BluePrint/GunSystem/BP_Magazine.Reload` (`self.Magazine`))
  (`/Game/BluePrint/system/BP_HPManager.HPInit` (`self.HPManager`) _output_get)
  (`self.StartPlayerTurn`)
  (`self.ShowBulletCount`))

(event `BulletClear`
  ; 弾を打ち尽くしたときに使用するカスタムイベント
  (`/Game/BluePrint/Item/BP_ItemManager.ReloadItem` (`self.ItemManager`) (`self.CurrentRound`))
  (`/Game/BluePrint/GunSystem/BP_Magazine.Reload` (`self.Magazine`))
  (`KismetSystemLibrary.Delay` 1.0)
  (`self.StartPlayerTurn`)
  (`self.ShowBulletCount`))

(event `StartPlayerTurn`
  (bind _inputstate (`self.InputState`))
  (set `/Game/BluePrint/system/InputState.CanInput` true _inputstate)
  (set `/Game/BluePrint/system/InputState.DamageValue` 1 _inputstate)
  (`self.SetInfoText` "プレイヤーのターン"))

(event `StartEnemyTurn`
  (bind _inputstate (`self.InputState`))
  (bind _hpmanager (`self.HPManager`))
  (bind _itemmanager (`self.ItemManager`))
  (bind _itemmanager_2 (`self.ItemManager`))
  (bind _inventoryenemy (`/Game/BluePrint/Item/BP_ItemManager.InventoryEnemy` _itemmanager_2))
  (`KismetSystemLibrary.Delay` 2.0)
  (if (`/Game/BluePrint/system/InputState.UseHandcuffsPlayer` _inputstate)
    (set `/Game/BluePrint/system/InputState.CanInput` true _inputstate)
    (set `/Game/BluePrint/system/InputState.UseHandcuffsPlayer` false _inputstate)
    (else
      (`self.SetInfoText` "ディーラーのターン")
      ; 敵の挙動
      (`KismetSystemLibrary.PrintString` "StartEnemyTurn")
      (if (> (`KismetArrayLibrary.Array_Length` (`/Game/BluePrint/Item/BP_ItemManager.InventoryEnemy` (`self.ItemManager`))) 0)
        (for _array_element (`/Game/BluePrint/Item/BP_ItemManager.InventoryEnemy` _itemmanager)
          (bind _asbp_cigarette (cast `/Game/BluePrint/Item/Items/BP_Cigarette` _array_element))
          (bind _output_get (set `self.HaveCigarette` true))
          (break))
        (if (and (!= (`/Game/BluePrint/system/BP_HPManager.EnemyHP` _hpmanager) (`/Game/BluePrint/system/BP_HPManager.EnemyCurrnentHP` _hpmanager)) _output_get)
          (`/Game/BluePrint/Item/BP_ItemManager.UseItemEnemy` _itemmanager _asbp_cigarette)
          (else
            (`/Game/BluePrint/Item/BP_ItemBase.UseItem` (`|GetArrayItem` _inventoryenemy (`KismetMathLibrary.RandomInteger` (`KismetArrayLibrary.Array_Length` _inventoryenemy))) false)
            (`/Game/BluePrint/Item/BP_ItemManager.UseItemEnemy` _itemmanager_2 null))))
      (`KismetSystemLibrary.Delay` 1.0)
      (bind (_onemoreturn _playerisdead _enemyisdead _lustbullet) (`self.ShotEnemy`))
      (if _onemoreturn
        (if _lustbullet
          (`self.StartRound`)
          (else
            (`self.StartEnemyTurn`)))
        (elif _playerisdead
          (goto _label)
          (elif _enemyisdead
            (goto _label_3)
            (elif _lustbullet
              (`self.StartRound`)
              (else
                (`self.StartPlayerTurn`)))))))))

(event `EnemyHPZero`
  (if (not (== (`self.MaxRound`) (`self.CurrentRound`)))
    (`self.StartRound`)))

(event `PlayerHPZero`)

(event `SetInfoText`
  (params (info :type String))
  (bind _asbp_uiplayer_controller (cast `/Game/BluePrint/system/BP_UIPlayerController` (`GameplayStatics.GetPlayerController` 0)))
  (bind _infotext (`/Game/BluePrint/system/WBP_InGameUI.InfoText` (`/Game/BluePrint/system/BP_UIPlayerController.InGameUI` _asbp_uiplayer_controller)))
  (set `TextBlock.Text` (`KismetTextLibrary.Conv_StringToText` info) _infotext)
  (`KismetSystemLibrary.Delay` 2.0)
  (set `TextBlock.Text` "" _infotext))

(event `ShowBulletCount`
  (bind (_bulletcount _blankcount) (`/Game/BluePrint/GunSystem/BP_Magazine.CountBullet` (`self.Magazine`)))
  (`self.SetInfoText` (`KismetStringLibrary.Concat_StrStr` (`KismetStringLibrary.Concat_StrStr` (`KismetStringLibrary.Concat_StrStr` (`KismetStringLibrary.Concat_StrStr` "実包" (`KismetStringLibrary.Conv_IntToString` _bulletcount)) "発、空砲は") (`KismetStringLibrary.Conv_IntToString` _blankcount)) "発だ...")))

(fn `ShotEnemy`
  (returns (OneMoreTurn :type Boolean) (PlayerIsDead :type Boolean) (EnemyIsDead :type Boolean) (LustBullet :type Boolean))
  (locals (OneMoerTurn :type Boolean) (PlayerDeadCheck :type Boolean) (EnemyDeadCheck :type Boolean))
  (bind _magazine (`self.Magazine`))
  (`KismetSystemLibrary.PrintString` "EnemyShotPlayer")
  (bind (_bulletcount _blankcount) (`/Game/BluePrint/GunSystem/BP_Magazine.CountBullet` _magazine))
  (bind (_bullet _lastbullet) (`/Game/BluePrint/GunSystem/BP_Magazine.GetNextBullet` _magazine))
  (if (>= _bulletcount _blankcount)
    ; プレイヤーに向けて射撃
    (if _bullet
      (`GameplayStatics.PlaySound2D` "/Game/Audio/Sound/拳銃を撃つ.拳銃を撃つ" 1.0 1.0 0.0 null null)
      (bind _isdead (`/Game/BluePrint/system/BP_HPManager.Damage` (`self.HPManager`) 0))
      (bind _asbp_uiplayer_controller (cast `/Game/BluePrint/system/BP_UIPlayerController` (`GameplayStatics.GetPlayerController` 0)))
      (set `local.PlayerDeadCheck` _isdead)
      (`/Game/BluePrint/system/BP_UIPlayerController.InvokeDamageEffect` _asbp_uiplayer_controller)
      (else
        (`GameplayStatics.PlaySound2D` "/Game/Audio/Sound/銃火器・空撃ち.銃火器・空撃ち" 1.0 1.0 0.0 null null)))
    (else
      ; 自分に向けて射撃
      (if _bullet
        (`GameplayStatics.PlaySound2D` "/Game/Audio/Sound/拳銃を撃つ.拳銃を撃つ" 1.0 1.0 0.0 null null)
        (bind _returnvalue (`GameplayStatics.GetActorOfClass` "/Game/BluePrint/Enemy/BP_Enemy.BP_Enemy_C"))
        (`/Game/BluePrint/Enemy/BP_Enemy.DamageReaction` _returnvalue)
        (bind _isdead_2 (`/Game/BluePrint/system/BP_HPManager.DamageEnemy` (`self.HPManager`) 0))
        (set `local.EnemyDeadCheck` _isdead_2)
        (else
          (set `local.OneMoerTurn` true)
          (`GameplayStatics.PlaySound2D` "/Game/Audio/Sound/銃火器・空撃ち.銃火器・空撃ち" 1.0 1.0 0.0 null null)))))
  (return (`local.OneMoerTurn`) (`local.PlayerDeadCheck`) (`local.EnemyDeadCheck`) _lastbullet))

(fn `UserConstructionScript`)