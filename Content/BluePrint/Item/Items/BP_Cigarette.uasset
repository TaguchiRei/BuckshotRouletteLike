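; BP_Cigarette is a usable item that restores one HP to whoever uses it, either the player or the enemy.
; It overrides UseItem, calling the parent first, then finds BP_HPManager in the level and uses the User boolean to choose HPUPPlayer or HPUPEnemy.
; It then sets FadeOut to true, while its event graph holds only disabled default events.
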(fn `UseItem`
  (params (User :type Boolean))
  (`parent.UseItem` User)
  (bind _returnvalue (`GameplayStatics.GetActorOfClass` "/Game/BluePrint/system/BP_HPManager.BP_HPManager_C"))
  (if User
    (`/Game/BluePrint/system/BP_HPManager.HPUPPlayer` _returnvalue 1)
    (else
      (`/Game/BluePrint/system/BP_HPManager.HPUPEnemy` _returnvalue 1)))
  (set `self.FadeOut` true))

(fn `UserConstructionScript`
  (`parent.UserConstructionScript`))