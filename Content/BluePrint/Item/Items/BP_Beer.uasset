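; BP_Beer is an item Blueprint that discards the next bullet from the gun's magazine and reveals whether it was live or blank.
; DisposeBullet takes the next bullet from BP_Magazine and writes the Japanese result message to the InfoText of the player controller's in-game UI.
; It then calls BulletClear on InGameState.
; A constant-true branch leaves the delayed fade-out and text clear unreachable.
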(event `DisposeBullet`
  (bind _returnvalue (`GameplayStatics.GetActorOfClass` "/Game/BluePrint/GunSystem/BP_Magazine.BP_Magazine_C"))
  (bind _bullet (`/Game/BluePrint/GunSystem/BP_Magazine.GetNextBullet` _returnvalue))
  (bind _asbp_uiplayer_controller (cast `/Game/BluePrint/system/BP_UIPlayerController` (`GameplayStatics.GetPlayerController` 0)))
  (if _bullet
    (bind _infotext (`/Game/BluePrint/system/WBP_InGameUI.InfoText` (`/Game/BluePrint/system/BP_UIPlayerController.InGameUI` _asbp_uiplayer_controller)))
    (set `TextBlock.Text` "捨てられた弾丸は実包だった..." _infotext)
    (else
      (set `TextBlock.Text` "捨てられた弾丸は空砲だった..." _infotext)))
  (if true
    (bind _asin_game_state (cast `/Game/BluePrint/system/InGameState` (`GameplayStatics.GetGameState`)))
    (`/Game/BluePrint/system/InGameState.BulletClear` _asin_game_state)
    (else
      (`KismetSystemLibrary.Delay` 1.5)
      (set `self.FadeOut` true)
      (set `TextBlock.Text` "" _infotext))))

(fn `UserConstructionScript`
  (`parent.UserConstructionScript`))