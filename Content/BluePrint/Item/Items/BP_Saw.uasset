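; Saw item Blueprint that, per its Japanese description, doubles the damage dealt for the current turn only.
; On BeginPlay it creates a dynamic material for the item and sets its display name and description.
; UseItem runs the parent logic, sets DamageValue on the InputState actor found by class lookup, then flags FadeOut.
; Tick defers to the parent, followed by an empty fade-time check; no turn-end reset appears here.
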(event `self.ReceiveBeginPlay`
  (`parent.ReceiveBeginPlay`)
  (`self.GenerateDynamicMat` (`self.Item`))
  (set `self.ItemName` "のこぎり")
  (set `self.ItemInfo` "そのターンのみ、与えるダメージが2倍になる"))

(event `self.ReceiveTick`
  (params (DeltaSeconds :type "Float (single-precision)"))
  (`parent.ReceiveTick` DeltaSeconds)
  (if (< (`self.FadeCurrentTime`) 0.0)
    _))

(fn `UseItem`
  (params (User :type Boolean))
  (`parent.UseItem` User)
  (bind _returnvalue (`GameplayStatics.GetActorOfClass` "/Game/BluePrint/system/InputState.InputState_C"))
  (set `/Game/BluePrint/system/InputState.DamageValue` 2 _returnvalue)
  (set `self.FadeOut` true))

(fn `UserConstructionScript`
  (`parent.UserConstructionScript`))