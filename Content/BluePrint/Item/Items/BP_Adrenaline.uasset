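; Adrenaline item that, per its description, lets the user steal and use an enemy's item.
; When UseItem passes a true User, it sets the InputState adrenaline flag, enables input, shifts the camera and moves the Wall aside.
; Tick polls that flag and, once cleared, restores the camera and the Wall position cached at BeginPlay, then sets FadeOut.
; A false User triggers no effect here.
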(event `self.ReceiveBeginPlay`
  (`parent.ReceiveBeginPlay`)
  (`self.GenerateDynamicMat` (`self.Item`))
  (set `self.ItemName` "アドレナリン")
  (set `self.ItemInfo` "敵のアイテムを奪って使用できる")
  (bind _returnvalue (`GameplayStatics.GetActorOfClass` "/Game/Art/Wall.Wall_C"))
  (set `self.WallLocation` (`self.K2_GetActorLocation` _returnvalue)))

(event `self.ReceiveTick`
  (params (DeltaSeconds :type "Float (single-precision)"))
  (`parent.ReceiveTick` DeltaSeconds)
  (if (== (`self.UsePlayer`) 0)
    _
    (elif (== (`self.UsePlayer`) 1)
      (bind _returnvalue (`GameplayStatics.GetActorOfClass` "/Game/BluePrint/system/InputState.InputState_C"))
      (if (not (`/Game/BluePrint/system/InputState.UseAdrenaline` _returnvalue))
        (bind _returnvalue_2 (`GameplayStatics.GetActorOfClass` "/Script/Engine.CameraActor"))
        (`self.K2_SetActorLocation` _returnvalue_2 (`self.OriginCameraVector`) false false)
        (bind _returnvalue_3 (`GameplayStatics.GetActorOfClass` "/Game/Art/Wall.Wall_C"))
        (`self.K2_SetActorLocation` _returnvalue_3 (`self.WallLocation`) false false)
        (set `self.FadeOut` true)))))

(event `UseAdrenaline`
  (params (User :type Boolean))
  (`GameplayStatics.GetActorOfClass` "/Game/Art/Wall.Wall_C")
  (bind _returnvalue (`GameplayStatics.GetActorOfClass` "/Game/BluePrint/system/InputState.InputState_C"))
  (if User
    (set `/Game/BluePrint/system/InputState.UseAdrenaline` true _returnvalue)
    (bind _returnvalue_2 (`GameplayStatics.GetActorOfClass` "/Script/Engine.CameraActor"))
    (`self.K2_SetActorLocation` _returnvalue_2 (`self.MovedCameraVector`) false false)
    (set `self.UsePlayer` 1)
    (set `/Game/BluePrint/system/InputState.CanInput` true _returnvalue)
    (bind _returnvalue_3 (`GameplayStatics.GetActorOfClass` "/Game/Art/Wall.Wall_C"))
    (`self.K2_SetActorLocation` _returnvalue_3 (999.0 999.0 99.0) false false)))

(fn `UseItem`
  (params (User :type Boolean))
  (`parent.UseItem` User)
  (`self.UseAdrenaline` User))

(fn `UserConstructionScript`
  (`parent.UserConstructionScript`))