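; BP_Handcuffs is a usable item that, per its description, blocks the opponent's turn for one turn.
; BeginPlay creates its dynamic material and sets the Japanese name and description.
; UseItem calls the parent, starts the fade-out, then finds the InputState actor and sets its player or enemy handcuffs flag from the User boolean.
; The turn skip itself is not implemented here.
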(event `self.ReceiveBeginPlay`
  (`parent.ReceiveBeginPlay`)
  (`self.GenerateDynamicMat` (`self.Item`))
  (set `self.ItemName` "手錠")
  (set `self.ItemInfo` "相手のターンを１ターン封じる"))

(fn `UseItem`
  (params (User :type Boolean))
  (`parent.UseItem` User)
  (set `self.FadeOut` true)
  (bind _returnvalue (`GameplayStatics.GetActorOfClass` "/Game/BluePrint/system/InputState.InputState_C"))
  (if User
    (set `/Game/BluePrint/system/InputState.UseHandcuffsPlayer` true _returnvalue)
    (else
      (set `/Game/BluePrint/system/InputState.UseHandcuffsEnemy` true _returnvalue))))

(fn `UserConstructionScript`
  (`parent.UserConstructionScript`))