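; BP_ItemBase is a base item Blueprint with a hover info display and a use notification.
; ItemInit copies the item's name and description into the WBP_ItemInfo instance held by its InfoWidget component.
; Cursor-over events on BoxCollision show and hide that widget.
; UseItem calls UsedEvent with itself as the argument, and ItemInit is not called within this graph.
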(event `ItemInit`
  (bind _aswbp_item_info (cast `/Game/BluePrint/Item/WBP_ItemInfo` (`WidgetComponent.GetUserWidgetObject` (`self.InfoWidget`))))
  (set `TextBlock.Text` (`KismetTextLibrary.Conv_StringToText` (`self.ItemName`)) (`/Game/BluePrint/Item/WBP_ItemInfo.ItemName` _aswbp_item_info))
  (set `TextBlock.Text` (`KismetTextLibrary.Conv_StringToText` (`self.ItemInfo`)) (`/Game/BluePrint/Item/WBP_ItemInfo.ItemInfo` _aswbp_item_info)))

(event `self.ReceiveBeginPlay`)

(event `ShowItemInfo`
  (`Widget.SetVisibility` (`WidgetComponent.GetUserWidgetObject` (`self.InfoWidget`)) "Visible"))

(event `HideItemInfo`
  (`Widget.SetVisibility` (`WidgetComponent.GetUserWidgetObject` (`self.InfoWidget`)) "Hidden"))

(event `self.BoxCollision.OnBeginCursorOver`
  (params (TouchedComponent :type "PrimitiveComponent Object Reference"))
  (`self.ShowItemInfo`))

(event `self.BoxCollision.OnEndCursorOver`
  (params (TouchedComponent :type "PrimitiveComponent Object Reference"))
  (`self.HideItemInfo`))

(fn `UseItem`
  (`self.UsedEvent` self))

(fn `UserConstructionScript`)