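; Item manager that spawns random items for the player and the enemy and tracks both inventories.
; Each item is picked from ItemList and assigned the first unused slot in its side's position list; player items spawn at SpawnPosition, enemy items at their slot.
; A used-event binding removes items from inventory, but slots are never freed.
; Per-round replacement clears inventory arrays without destroying actors, and a reload event adds more items.
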(event `self.ReceiveBeginPlay`
  ; 開始時の処理
  (for (_array_element _array_index) (`self.MaxItemNum`)
    (if (> _array_element (`KismetArrayLibrary.Array_Length` (`self.SetPositionListPlayer`)))
      (`KismetSystemLibrary.PrintString` (`KismetStringLibrary.Concat_StrStr` (`KismetStringLibrary.Concat_StrStr` "MaxItemNumの" (`KismetStringLibrary.Conv_IntToString` _array_index)) "番目はSetPositionListの長さより多い数値が設定されています")))))

(event `AddItemPlayer`
  (params (ItemType :type "/Game/BluePrint/Item/BP_ItemBase Object Reference"))
  (bind _usedsetposplayer (`self.UsedSetPosPlayer`))
  ; プレイヤー用アイテムの追加処理
  (bind _returnvalue (`|SpawnActorFromClass` (`GameplayStatics.GetObjectClass` ItemType) (`KismetMathLibrary.Conv_VectorToTransform` (`self.SpawnPosition`)) "Undefined" "MultiplyWithRoot" null null))
  (`KismetArrayLibrary.Array_Add` (`self.InventoryPlayer`) _returnvalue)
  (for _index (range (+ (`KismetArrayLibrary.Array_Length` (`self.SetPositionListPlayer`)) 1))
    ;; ループ内処理　//設置可能位置からまだ使われていない個所を探す
    (if (not (`KismetArrayLibrary.Array_Contains` _usedsetposplayer _index))
      (bind _returnvalue_2 (`KismetArrayLibrary.Array_Add` _usedsetposplayer _index))
      (break)))
  (set `/Game/BluePrint/Item/BP_ItemBase.SetPosition` (`|GetArrayItem` (`self.SetPositionListPlayer`) _returnvalue_2) _returnvalue)
  ; アイテム使用時のイベントを登録
  (add `/Game/BluePrint/Item/BP_ItemBase.UsedEvent` _returnvalue (delegate `UsedEventPlayer`)))

(event `UsedEventPlayer`
  (params (ItemInstance :type "/Game/BluePrint/Item/BP_ItemBase Object Reference"))
  ; アイテム使用時のイベントを登録
  (`self.UseItemPlayer` ItemInstance))

(event `AddItemEnemy`
  (params (ItemType :type "/Game/BluePrint/Item/BP_ItemBase Object Reference"))
  (bind _usedsetposenemy (`self.UsedSetPosEnemy`))
  ; 敵用アイテムの追加処理
  (for _index (range (+ (`KismetArrayLibrary.Array_Length` (`self.SetPositionListPlayer`)) 1))
    ;; ループ内処理　//設置可能位置からまだ使われていない個所を探す
    (if (not (`KismetArrayLibrary.Array_Contains` _usedsetposenemy _index))
      (bind _returnvalue (`KismetArrayLibrary.Array_Add` _usedsetposenemy _index))
      (break)))
  (bind _output (`|GetArrayItem` (`self.SetPositionListEnemy`) _returnvalue))
  (bind _returnvalue_2 (`|SpawnActorFromClass` (`GameplayStatics.GetObjectClass` ItemType) (`KismetMathLibrary.Conv_VectorToTransform` _output) "Undefined" "MultiplyWithRoot" null null))
  (`KismetArrayLibrary.Array_Add` (`self.InventoryEnemy`) _returnvalue_2)
  (set `/Game/BluePrint/Item/BP_ItemBase.SetPosition` _output _returnvalue_2)
  ; アイテム使用時のイベントを登録
  (add `/Game/BluePrint/Item/BP_ItemBase.UsedEvent` _returnvalue_2 (delegate `UsedEvent_Enemy`)))

(event `UsedEvent_Enemy`
  (params (ItemInstance :type "/Game/BluePrint/Item/BP_ItemBase Object Reference"))
  ; アイテム使用時のイベントを登録
  (`self.UseItemEnemy` ItemInstance))

(event `ReplaceAllItem`
  (params (Round :type Integer))
  ; アイテムをすべて置き換える
  (`KismetArrayLibrary.Array_Clear` (`self.InventoryPlayer`))
  (`KismetArrayLibrary.Array_Clear` (`self.InventoryEnemy`))
  (for _ (range (+ (- (`|GetArrayItem` (`self.MaxItemNum`) Round) 0) 1))
    (bind _selecteditem (`self.SelectRandomItem`))
    (`self.AddItemPlayer` _selecteditem)
    (bind _selecteditem_2 (`self.SelectRandomItem`))
    (`self.AddItemEnemy` _selecteditem_2)))

(event `ReloadItem`
  ; アイテムの補充を行う
  (for _ (range (`KismetMathLibrary.And_IntInt` (- (`|GetArrayItem` (`self.MaxItemNum`)) 0) (`KismetArrayLibrary.Array_Length` (`self.SetPositionListPlayer`))))
    (bind _selecteditem (`self.SelectRandomItem`))
    (`self.AddItemPlayer` _selecteditem))
  (for _ (range (`KismetMathLibrary.And_IntInt` (- (`|GetArrayItem` (`self.MaxItemNum`)) 0) (`KismetArrayLibrary.Array_Length` (`self.SetPositionListEnemy`))))
    (bind _selecteditem_2 (`self.SelectRandomItem`))
    (`self.AddItemEnemy` _selecteditem_2)))

(event `UseItemPlayer`
  (params (UsedItem :type "/Game/BluePrint/Item/BP_ItemBase Object Reference"))
  ; プレイヤーアイテムの使用
  (if (`KismetArrayLibrary.Array_Contains` (`self.InventoryPlayer`) UsedItem)
    (`KismetArrayLibrary.Array_RemoveItem` (`self.InventoryPlayer`) UsedItem)))

(event `UseItemEnemy`
  (params (UsedItem :type "/Game/BluePrint/Item/BP_ItemBase Object Reference"))
  ; 敵アイテムの使用
  (if (`KismetArrayLibrary.Array_Contains` (`self.InventoryEnemy`) UsedItem)
    (`KismetArrayLibrary.Array_RemoveItem` (`self.InventoryEnemy`) UsedItem)))

(fn `SelectRandomItem`
  (returns (SelectedItem :type "/Game/BluePrint/Item/BP_ItemBase Object Reference"))
  (return (`|GetArrayItem` (`self.ItemList`) (`KismetMathLibrary.RandomInteger` (`KismetArrayLibrary.Array_Length` (`self.ItemList`))))))

(fn `UserConstructionScript`
  (locals (UsePosition :type "Array of Integer")))